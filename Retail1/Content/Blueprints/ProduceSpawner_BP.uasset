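; ProduceSpawner_BP is a produce spawner actor that shows an interaction progress bar.
; Each Tick, it sets the ProgressBar widget component's visibility from CanInteract.
; While interactable with a positive TimeToComplete, it passes Progress and TimeToComplete to the bar's ItemWidget_BP through SetCleanupProgress.
; The Blueprint only handles this display, with no spawning or progress logic in its graphs.
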(event EventBeginPlay)

(event Collision|EventActorBeginOverlap
  (params (OtherActor :type Actor%20Object%20Reference)))

(event EventTick
  (params (DeltaSeconds :type Float%20%28single-precision%29))
  (bind _caninteract (Variables|Default|GetcanInteract))
  (bind _progressbar (Variables|Default|GetProgressBar))
  (bind _timetocomplete (Variables|Default|GettimeToComplete))
  (Rendering|SetVisibility _progressbar _caninteract false)
  (if _caninteract
    (bind _asitem_widget_bp (Utilities|Casting|CastToItemWidget_BP (UserInterface|GetUserWidgetObject _progressbar)))
    (if (> _timetocomplete 0.0)
      (Default|SetCleanupProgress _asitem_widget_bp (Variables|Default|Getprogress) _timetocomplete))))

(fn ConstructionScript)