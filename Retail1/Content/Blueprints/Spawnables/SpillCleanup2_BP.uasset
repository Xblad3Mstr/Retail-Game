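; SpillCleanup2_BP is a spawnable spill cleanup actor that displays cleanup progress on two widget-based progress bars.
; Every tick it casts both widget components to CleanupWidget_BP and passes them Progress and TimeToComplete, printing a debug string when a cast or time check fails.
; The second bar updates only after the first succeeds, and nothing in these graphs changes Progress itself.
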(event EventBeginPlay)

(event Collision|EventActorBeginOverlap
  (params (OtherActor :type Actor%20Object%20Reference)))

(event EventTick
  (params (DeltaSeconds :type Float%20%28single-precision%29))
  (bind _timetocomplete (Variables|Default|GettimeToComplete))
  (bind _timetocomplete_2 (Variables|Default|GettimeToComplete))
  (bind _ascleanup_widget_bp (Utilities|Casting|CastToCleanupWidget_BP (UserInterface|GetUserWidgetObject (Variables|Default|GetProgressBar)))
    (:then
      (if (> _timetocomplete_2 0.0)
        (Default|SetCleanupProgress _ascleanup_widget_bp (Variables|Default|Getprogress) _timetocomplete_2)
        (bind _ascleanup_widget_bp_2 (Utilities|Casting|CastToCleanupWidget_BP (UserInterface|GetUserWidgetObject (Variables|Default|GetProgressBar1)))
          (:then
            (if (> _timetocomplete 0.0)
              (Default|SetCleanupProgress _ascleanup_widget_bp_2 (Variables|Default|Getprogress) _timetocomplete)
              (else
                (Development|PrintString "\"Something Else Failed\""))))
          (:CastFailed
            (Development|PrintString "\"Something Failed\"")))
        (else
          (Development|PrintString "\"Something Else Failed\""))))
    (:CastFailed
      (Development|PrintString "\"Something Failed\""))))

(fn ConstructionScript)