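; InteractablePinkCustomer_BP is an interactable customer that shows item icons on two widget components, presumably the items it wants.
; While TimerStarted is true, Tick casts both widgets to CustomerWidget_BP, calls SetTextVisibility and sets each icon from its own GetItem call.
; The second widget updates only if the first cast succeeds, and failed casts print a debug string.
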(event EventBeginPlay)

(event Collision|EventActorBeginOverlap
  (params (OtherActor :type Actor%20Object%20Reference)))

(event EventTick
  (params (DeltaSeconds :type Float%20%28single-precision%29))
  (if (Variables|Default|GettimerStarted)
    (bind _ascustomer_widget_bp (Utilities|Casting|CastToCustomerWidget_BP (UserInterface|GetUserWidgetObject (Variables|Default|GetWidget)))
      (:then
        (bind _returnvalue (Class|Customer|GetItem))
        (Default|SetTextVisibility _ascustomer_widget_bp)
        (Default|SetIconImage _ascustomer_widget_bp _returnvalue)
        (bind _ascustomer_widget_bp_2 (Utilities|Casting|CastToCustomerWidget_BP (UserInterface|GetUserWidgetObject (Variables|Default|GetWidget1)))
          (:then
            (bind _returnvalue_2 (Class|Customer|GetItem))
            (Default|SetTextVisibility _ascustomer_widget_bp_2)
            (Default|SetIconImage _ascustomer_widget_bp_2 _returnvalue_2))
          (:CastFailed
            (Development|PrintString "\"Customer Widget Cast Failed"))))
      (:CastFailed
        (Development|PrintString "\"Cast Failed\"")))))

(fn ConstructionScript)