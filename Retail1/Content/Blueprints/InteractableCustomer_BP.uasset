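; InteractableCustomer_BP is a customer Blueprint that displays an item icon on its widgets.
; On BeginPlay it casts the user objects of two widget components, Widget and Widget1, to CustomerWidget_BP and passes each a GetItem result through SetIconImage.
; The second widget is handled only if the first cast succeeds, and failed casts print debug strings.
; Tick, overlap and the construction script are empty.
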(event EventBeginPlay
  (bind _ascustomer_widget_bp (Utilities|Casting|CastToCustomerWidget_BP (UserInterface|GetUserWidgetObject (Variables|Default|GetWidget)))
    (:then
      (bind _returnvalue (Class|Customer|GetItem))
      (Default|SetIconImage _ascustomer_widget_bp _returnvalue)
      (bind _ascustomer_widget_bp_2 (Utilities|Casting|CastToCustomerWidget_BP (UserInterface|GetUserWidgetObject (Variables|Default|GetWidget1)))
        (:then
          (bind _returnvalue_2 (Class|Customer|GetItem)))
        (:CastFailed
          (Development|PrintString "\"Customer Widget Cast Failed")))
      (Default|SetIconImage _ascustomer_widget_bp_2 _returnvalue_2))
    (:CastFailed
      (Development|PrintString "\"Cast Failed\""))))

(event Collision|EventActorBeginOverlap
  (params (OtherActor :type Actor%20Object%20Reference)))

(event EventTick
  (params (DeltaSeconds :type Float%20%28single-precision%29)))

(fn ConstructionScript)